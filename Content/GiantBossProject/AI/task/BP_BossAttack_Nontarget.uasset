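; Behavior Tree task that makes BP_Giant play a boss attack montage without targeting.
; It measures the giant's distance to the player, then picks a random montage from the "behind" set within 400 units or the "nontarget" set otherwise.
; When the montage completes it calls HitPlayer and finishes; a failed giant cast fails the task.
; All hit functions are empty, with HitPlayer's sphere-trace damage logic left disconnected.
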(event EventReceiveExecuteAI
  (params (OwnerController :type AI%20Controller%20Object%20Reference) (ControlledPawn :type Pawn%20Object%20Reference))
  (Variables|Default|SetControlledPawn ControlledPawn)
  (bind _asbp_giant (Utilities|Casting|CastToBP_Giant ControlledPawn)
    (:then
      (Variables|Default|Setintermediate_distance (Math|Vector|VectorLength (- (Transformation|GetActorLocation _asbp_giant) (Transformation|GetActorLocation (Game|Player|GetPlayerPawn 0)))))
      (if (<= (Variables|Default|Getintermediate_distance) 4e+02)
        (Animation|Montage|PlayMontage (Variables|/Script/Engine.Character|GetMesh _asbp_giant) (.OutItem (Utilities|Array|Random (Variables|Default|GetMontage%20to%20Play_Behind)))
          (:OnCompleted
            (CallFunction|HitPlayer)))
        (else
          (Animation|Montage|PlayMontage (Variables|/Script/Engine.Character|GetMesh _asbp_giant) (.OutItem (Utilities|Array|Random (Variables|Default|GetMontage%20to%20Play_Nontarget)))
            (:OnCompleted
              (CallFunction|HitPlayer)))))
      (AI|BehaviorTree|FinishExecute true))
    (:CastFailed
      (AI|BehaviorTree|FinishExecute false))))

(fn HitPlayer)

(fn HitBehind)

(fn HitShock)

(fn HitThrow)

(fn HitDouble)

(fn HitTriple)