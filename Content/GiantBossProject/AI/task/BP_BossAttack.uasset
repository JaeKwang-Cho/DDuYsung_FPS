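; Behavior tree task that makes BP_Giant play an attack montage, apparently in a test state.
; It plays montages from a test array in index order without wrapping, finishing on completion or failing if the pawn is not a giant.
; Player distance is computed but unused, as the range-based shock attack branch is disconnected.
; All hit functions are empty, with HitPlayer's sphere-trace damage logic left unwired.
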(event EventReceiveExecuteAI
  (params (OwnerController :type AI%20Controller%20Object%20Reference) (ControlledPawn :type Pawn%20Object%20Reference))
  (bind _montage_to_play_test (Variables|Default|GetMontage%20to%20Play_Test))
  (bind _testindex (Variables|Default|GetTestIndex))
  (bind _output (Utilities|Array|Get(acopy) _montage_to_play_test _testindex))
  (Variables|Default|SetControlledPawn ControlledPawn)
  (bind _asbp_giant (Utilities|Casting|CastToBP_Giant ControlledPawn)
    (:then
      (Variables|Default|Setintermediate_distance (Math|Vector|VectorLength (- (Transformation|GetActorLocation _asbp_giant) (Transformation|GetActorLocation (Game|Player|GetPlayerPawn 0)))))
      (Animation|Montage|PlayMontage (Variables|/Script/Engine.Character|GetMesh _asbp_giant) _output
        (:OnCompleted
          (Math|Integer|IncrementInt (Variables|Default|GetTestIndex)
            (:%20%20
              (Development|PrintString (Utilities|GetDisplayName _output))
              (CallFunction|HitPlayer)
              (AI|BehaviorTree|FinishExecute true))))))
    (:CastFailed
      (AI|BehaviorTree|FinishExecute false))))

(fn HitPlayer)

(fn HitBehind)

(fn HitShock)

(fn HitThrow)

(fn HitDouble)

(fn HitTriple)