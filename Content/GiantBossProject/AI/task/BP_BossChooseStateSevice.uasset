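; Behavior tree service that chooses the giant boss's combat state from its health and its distance to the player.
; Each AI tick sets the low-health blackboard flag when BP_Giant drops below half health.
; It also writes a state enum for far, mid or close range.
; The far branch sits behind a DoOnce with no visible reset, so it disables controller yaw and sets its state only once.
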(event EventReceiveTickAI
  (params (OwnerController :type AI%20Controller%20Object%20Reference) (ControlledPawn :type Pawn%20Object%20Reference) (DeltaSeconds :type Float%20%28single-precision%29))
  (bind _bb_lowhealth (Variables|Default|Getbb_lowhealth))
  (Variables|Default|SetControlledPawn ControlledPawn)
  (bind _percent (Default|GetPercentOfHealth (.AsBP%20Giant (Utilities|Casting|CastToBP_Giant (Variables|Default|GetControlledPawn)))))
  (if (< _percent 0.5)
    (Class|BTFunctionLibrary|SetBlackboardValueasBool _bb_lowhealth true)
    (else
      (Class|BTFunctionLibrary|SetBlackboardValueasBool _bb_lowhealth false)))
  (if (>= (Math|Vector|VectorLength (- (Transformation|GetActorLocation (Variables|Default|GetControlledPawn)) (Transformation|GetActorLocation (Game|Player|GetPlayerPawn 0)))) 3e+03)
    (Utilities|FlowControl|DoOnce false
      (:Completed
        (Variables|/Script/Engine.Pawn|SetbUseControllerRotationYaw (Variables|Default|GetControlledPawn) false)
        (AI|Components|Blackboard|SetValueasEnum (AI|GetBlackboard (Variables|Default|GetControlledPawn)) (Variables|Default|GetKeyName))))
    (elif (Math|Float|InRange(Float) (Math|Vector|VectorLength (- (Transformation|GetActorLocation (Variables|Default|GetControlledPawn)) (Transformation|GetActorLocation (Game|Player|GetPlayerPawn 0)))) 0.0 7e+02)
      (AI|Components|Blackboard|SetValueasEnum (AI|GetBlackboard (Variables|Default|GetControlledPawn)) (Variables|Default|GetKeyName) 2)
      (else
        (AI|Components|Blackboard|SetValueasEnum (AI|GetBlackboard (Variables|Default|GetControlledPawn)) (Variables|Default|GetKeyName) 1)))))