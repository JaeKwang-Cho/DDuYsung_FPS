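; Behavior tree task that runs the giant boss's non-focus attack.
; It plays a random montage from the shock set on BP_Giant, then finishes successfully on completion, or fails if the pawn is not a giant.
; Player distance is computed, but its range branch is disconnected.
; All hit functions are empty stubs, with HitPlayer's sphere trace and damage logic left unwired, so the task deals no damage itself.
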(event EventReceiveExecuteAI
  (params (OwnerController :type AI%20Controller%20Object%20Reference) (ControlledPawn :type Pawn%20Object%20Reference))
  (bind _montage_to_play_shock (Variables|Default|GetMontage%20to%20Play_Shock))
  (Development|PrintString "non focus")
  (bind _output_get (Variables|Default|SetControlledPawn ControlledPawn))
  (bind _asbp_giant (Utilities|Casting|CastToBP_Giant _output_get)
    (:then
      (Variables|Default|Setintermediate_distance (Math|Vector|VectorLength (- (Transformation|GetActorLocation _asbp_giant) (Transformation|GetActorLocation (Game|Player|GetPlayerPawn 0)))))
      (Animation|Montage|PlayMontage (Variables|/Script/Engine.Character|GetMesh _asbp_giant) (.OutItem (Utilities|Array|Random _montage_to_play_shock))
        (:OnCompleted
          (Math|Integer|IncrementInt (Variables|Default|GetTestIndex)
            (:%20%20
              (Development|PrintString (Utilities|GetDisplayName (Utilities|Array|Get(acopy) _montage_to_play_shock (Variables|Default|GetTestIndex))))
              (CallFunction|HitPlayer)
              (AI|BehaviorTree|FinishExecute true))))))
    (:CastFailed
      (AI|BehaviorTree|FinishExecute false))))

(fn HitPlayer)

(fn HitBehind)

(fn HitShock)

(fn HitThrow)

(fn HitDouble)

(fn HitTriple)