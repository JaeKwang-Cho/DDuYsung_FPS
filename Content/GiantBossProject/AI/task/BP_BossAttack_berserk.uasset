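; Behavior tree task for the giant boss's berserk attack.
; On AI execute it casts the pawn to BP_Giant, plays a random montage from the berserk list, and finishes successfully when the montage completes.
; HitPlayer is called on completion but is empty; its sphere trace and damage nodes are disconnected, so the task deals no damage.
; No other montage outcome, such as interruption, finishes the task.
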(event EventReceiveExecuteAI
  (params (OwnerController :type AI%20Controller%20Object%20Reference) (ControlledPawn :type Pawn%20Object%20Reference))
  (Variables|Default|SetControlledPawn ControlledPawn)
  (bind _asbp_giant (Utilities|Casting|CastToBP_Giant ControlledPawn))
  (Animation|Montage|PlayMontage (Variables|/Script/Engine.Character|GetMesh _asbp_giant) (.OutItem (Utilities|Array|Random (Variables|Default|GetMontage%20to%20Play_Berserk)))
    (:OnCompleted
      (CallFunction|HitPlayer)
      (AI|BehaviorTree|FinishExecute true))))

(fn HitPlayer)