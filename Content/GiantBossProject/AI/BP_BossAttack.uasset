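; Behavior tree task that makes BP_Giant attack, choosing by its distance to the player pawn.
; Within 700 units it plays a random hit montage, otherwise a random throw montage.
; The montage's first notify calls HitPlayer and finishes the task successfully; a failed Giant cast fails it.
; HitPlayer and the other hit functions are empty stubs, with HitPlayer's sphere-trace damage logic left disconnected.
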(event EventReceiveExecuteAI
  (params (OwnerController :type AI%20Controller%20Object%20Reference) (ControlledPawn :type Pawn%20Object%20Reference))
  (Variables|Default|SetControlledPawn ControlledPawn)
  (bind _asbp_giant (Utilities|Casting|CastToBP_Giant ControlledPawn)
    (:then
      (Variables|Default|Setintermediate_distance (Math|Vector|VectorLength (- (Transformation|GetActorLocation _asbp_giant) (Transformation|GetActorLocation (Game|Player|GetPlayerPawn 0)))))
      (if (<= (Variables|Default|Getintermediate_distance) 7e+02)
        (bind _notifyname (Animation|Montage|PlayMontage (Variables|/Script/Engine.Character|GetMesh _asbp_giant) (.OutItem (Utilities|Array|Random (Variables|Default|GetMontage%20to%20Play_Hit))))
          (:OnNotifyBegin
            (Development|PrintString (Utilities|String|ToString(Name) _notifyname))
            (CallFunction|HitPlayer)))
        (else
          (bind _notifyname_2 (Animation|Montage|PlayMontage (Variables|/Script/Engine.Character|GetMesh _asbp_giant) (.OutItem (Utilities|Array|Random (Variables|Default|GetMontage%20to%20Play_Throw))))
            (:OnNotifyBegin
              (Development|PrintString (Utilities|String|ToString(Name) _notifyname_2))
              (CallFunction|HitPlayer)))))
      (AI|BehaviorTree|FinishExecute true))
    (:CastFailed
      (AI|BehaviorTree|FinishExecute false))))

(fn HitPlayer)

(fn HitBehind)

(fn HitShock)

(fn HitThrow)

(fn HitDouble)

(fn HitTriple)