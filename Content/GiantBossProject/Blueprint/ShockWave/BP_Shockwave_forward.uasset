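; Forward-moving shockwave actor that damages the FPS player character, apparently a boss attack.
; A looping timer repeatedly scales WaveBox up on Z and steps it along its relative X axis without sweeping, so the wave grows as it travels.
; Overlaps with BP_FPS_Character apply damage using the DBP_ShowWave_f damage type.
; The actor destroys itself after a short fixed lifetime.
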(event OnComponentBeginOverlap(WaveBox)
  (params (OverlappedComponent :type Primitive%20Component%20Object%20Reference) (OtherActor :type Actor%20Object%20Reference) (OtherComp :type Primitive%20Component%20Object%20Reference) (OtherBodyIndex :type Integer) (bFromSweep :type Boolean) (SweepResult :type Hit%20Result%20Structure%20%28by%20ref%29))
  (bind _asbp_fps_character (Utilities|Casting|CastToBP_FPS_Character OtherActor))
  (Game|Damage|ApplyDamage _asbp_fps_character 1.0 0 0 "/Game/Blueprints/Damage/Damage_Giant/DBP_ShowWave_f.DBP_ShowWave_f_C"))

(event Custom|doShowWave
  (bind _wavebox (Variables|Default|GetWaveBox))
  (bind _returnvalue (Transformation|GetWorldScale _wavebox))
  (bind _relativelocation (Variables|/Script/Engine.SceneComponent|GetRelativeLocation _wavebox))
  (bind (_x _y _z) (Math|Vector|BreakVector _relativelocation))
  (bind (_x_2 _y_2 _z_2) (Math|Vector|BreakVector _returnvalue))
  (Transformation|SetWorldScale3D _wavebox (Math|Vector|MakeVector _x_2 _y_2 (* _z_2 1.1)))
  (Transformation|SetRelativeLocation (Variables|Default|GetWaveBox) (Math|Vector|MakeVector (+ _x 25.0) _y _z) false false))

(event EventBeginPlay
  (Utilities|Time|SetTimerbyEvent (delegate Custom|doShowWave) 0.03 true)
  (Utilities|FlowControl|Delay 1.5)
  (Actor|DestroyActor))

(fn ConstructionScript)