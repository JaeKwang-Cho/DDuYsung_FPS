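; BP_Shockwave is a short-lived expanding shockwave actor that damages BP_FirstPersonCharacter on contact.
; A looping timer started on BeginPlay scales OuterRing geometrically in X and Y and grows InnerRing by the same absolute step, preserving their scale difference and leaving Z unchanged.
; Begin-overlap on either ring independently applies damage to the character.
; The actor destroys itself after one second.
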(event OnComponentBeginOverlap(OuterRing)
  (params (OverlappedComponent :type Primitive%20Component%20Object%20Reference) (OtherActor :type Actor%20Object%20Reference) (OtherComp :type Primitive%20Component%20Object%20Reference) (OtherBodyIndex :type Integer) (bFromSweep :type Boolean) (SweepResult :type Hit%20Result%20Structure%20%28by%20ref%29))
  (bind _asbp_first_person_character (Utilities|Casting|CastToBP_FirstPersonCharacter OtherActor))
  (Game|Damage|ApplyDamage _asbp_first_person_character 1.0 0 0))

(event OnComponentBeginOverlap(InnerRing)
  (params (OverlappedComponent :type Primitive%20Component%20Object%20Reference) (OtherActor :type Actor%20Object%20Reference) (OtherComp :type Primitive%20Component%20Object%20Reference) (OtherBodyIndex :type Integer) (bFromSweep :type Boolean) (SweepResult :type Hit%20Result%20Structure%20%28by%20ref%29))
  (bind _asbp_first_person_character (Utilities|Casting|CastToBP_FirstPersonCharacter OtherActor))
  (Game|Damage|ApplyDamage _asbp_first_person_character 1.0 0 0))

(event Custom|doShowWave
  (bind _innerring (Variables|Default|GetInnerRing))
  (bind _outerring (Variables|Default|GetOuterRing))
  (bind _returnvalue (Transformation|GetWorldScale _outerring))
  (bind _returnvalue_2 (Transformation|GetWorldScale _innerring))
  (bind (_x _y _z) (Math|Vector|BreakVector _returnvalue))
  (bind (_x_2 _y_2 _z_2) (Math|Vector|BreakVector _returnvalue_2))
  (bind _returnvalue_3 (* _returnvalue 1.05))
  (bind _x_3 (Math|Vector|BreakVector _returnvalue_3))
  (bind _returnvalue_4 (- _x_3 _x))
  (bind _returnvalue_5 (+ _x_2 _returnvalue_4))
  (Transformation|SetWorldScale3D _innerring (Math|Vector|MakeVector _returnvalue_5 _returnvalue_5 _z_2))
  (Transformation|SetWorldScale3D _outerring (Math|Vector|MakeVector _x_3 _x_3 _z)))

(event EventBeginPlay
  (Utilities|Time|SetTimerbyEvent (delegate Custom|doShowWave) 0.03 true)
  (Utilities|FlowControl|Delay 1.0)
  (Actor|DestroyActor))

(fn ConstructionScript)