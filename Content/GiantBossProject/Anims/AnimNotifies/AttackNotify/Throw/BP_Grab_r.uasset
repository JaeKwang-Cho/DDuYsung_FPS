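; Anim notify state "grabNThrow" for a right-hand grab attack that catches the first-person player character.
; On begin, a sphere overlap at the hand socket flags a grab in GI_GameInstance, stores the mesh's right vector as FrontVector and calls CallLevelStartGrab.
; While grabbed, each tick passes the socket location to CallCharSetRocation through the game instance.
; Notify end does nothing, so the release is not handled here.
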(fn ReceivedNotifyBegin
  (params (MeshComp :type Skeletal%20Mesh%20Component%20Object%20Reference) (Animation :type Anim%20Sequence%20Base%20Object%20Reference) (TotalDuration :type Float%20%28single-precision%29) (EventReference :type Anim%20Notify%20Event%20Reference%20Structure%20%28by%20ref%29))
  (bind _returnvalue (Collision|SphereOverlapActors MeshComp (Transformation|GetSocketLocation MeshComp "hand_rSocket") 2e+02 (Utilities|Array|MakeArray "ObjectTypeQuery3") "/Game/Blueprints/FirstPerson/BP_FirstPersonCharacter.BP_FirstPersonCharacter_C"))
  (if _returnvalue
    (bind _asgi_game_instance (Utilities|Casting|CastToGI_GameInstance (Game|GetGameInstance MeshComp)))
    (Variables|/Game/GiantBossProject/Blueprint/GI_GameInstance.GI_GameInstance_C|SetFrontVector _asgi_game_instance (Math|Vector|GetRightVector MeshComp))
    (bind _output_get (Variables|/Game/GiantBossProject/Blueprint/GI_GameInstance.GI_GameInstance_C|SetbGrabbed _asgi_game_instance _returnvalue))
    (Default|CallLevelStartGrab _asgi_game_instance)
    (return _output_get)))

(fn ReceivedNotifyTick
  (params (MeshComp :type Skeletal%20Mesh%20Component%20Object%20Reference) (Animation :type Anim%20Sequence%20Base%20Object%20Reference) (FrameDeltaTime :type Float%20%28single-precision%29) (EventReference :type Anim%20Notify%20Event%20Reference%20Structure%20%28by%20ref%29))
  (bind _asgi_game_instance (Utilities|Casting|CastToGI_GameInstance (Game|GetGameInstance MeshComp)))
  (if (Variables|/Game/GiantBossProject/Blueprint/GI_GameInstance.GI_GameInstance_C|GetbGrabbed _asgi_game_instance)
    (bind _output_get (Variables|/Game/GiantBossProject/Blueprint/GI_GameInstance.GI_GameInstance_C|SetSocketTransform _asgi_game_instance (Transformation|GetSocketTransform MeshComp "hand_rSocket" "RTS_World")))
    (Default|CallCharSetRocation _asgi_game_instance (.location _output_get))
    (return (Variables|/Game/GiantBossProject/Blueprint/GI_GameInstance.GI_GameInstance_C|GetbGrabbed _asgi_game_instance))))

(fn ReceivedNotifyEnd
  (params (MeshComp :type Skeletal%20Mesh%20Component%20Object%20Reference) (Animation :type Anim%20Sequence%20Base%20Object%20Reference) (EventReference :type Anim%20Notify%20Event%20Reference%20Structure%20%28by%20ref%29))
  (return false))

(fn GetNotifyName
  (return "grabNThrow"))