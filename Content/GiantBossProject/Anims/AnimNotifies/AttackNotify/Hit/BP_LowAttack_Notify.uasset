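; BP_LowAttack_Notify is an animation notify state, displayed as "LowAttack", that deals hit damage to the player during an attack animation.
; Each tick it sphere-overlaps pawns around the mesh's right-hand socket, filtered to BP_FirstPersonCharacter.
; It applies DBP_Hit damage to the first match and returns, with no guard against repeat hits on later ticks.
; Begin and end do nothing.
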(fn ReceivedNotifyBegin
  (params (MeshComp :type Skeletal%20Mesh%20Component%20Object%20Reference) (Animation :type Anim%20Sequence%20Base%20Object%20Reference) (TotalDuration :type Float%20%28single-precision%29) (EventReference :type Anim%20Notify%20Event%20Reference%20Structure%20%28by%20ref%29))
  (return false))

(fn ReceivedNotifyTick
  (params (MeshComp :type Skeletal%20Mesh%20Component%20Object%20Reference) (Animation :type Anim%20Sequence%20Base%20Object%20Reference) (FrameDeltaTime :type Float%20%28single-precision%29) (EventReference :type Anim%20Notify%20Event%20Reference%20Structure%20%28by%20ref%29))
  (bind _outactors (Collision|SphereOverlapActors MeshComp (Transformation|GetSocketLocation MeshComp "hand_rSocket") 1e+02 (Utilities|Array|MakeArray "ObjectTypeQuery3") "/Game/Blueprints/FirstPerson/BP_FirstPersonCharacter.BP_FirstPersonCharacter_C"))
  (for _array_element _outactors
    (Game|Damage|ApplyDamage _array_element 1.0 0 0 "/Game/Blueprints/Damage/Damage_Giant/DBP_Hit.DBP_Hit_C")
    (return false)))

(fn ReceivedNotifyEnd
  (params (MeshComp :type Skeletal%20Mesh%20Component%20Object%20Reference) (Animation :type Anim%20Sequence%20Base%20Object%20Reference) (EventReference :type Anim%20Notify%20Event%20Reference%20Structure%20%28by%20ref%29))
  (return false))

(fn GetNotifyName
  (return "LowAttack"))