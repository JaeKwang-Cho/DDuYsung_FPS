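; Anim notify state for a right-hand hit in a boss attack, named DoubleMediumAttack_2, that knocks back the player character.
; Each tick sphere-checks pawns around hand_rSocket for BP_FPS_Character.
; A hit launches the character horizontally away from the hand with a fixed lift, then calls ApplyDamage with DBP_Hit but no damaged actor set.
; No guard prevents repeat hits on later ticks.
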(fn ReceivedNotifyBegin
  (params (MeshComp :type Skeletal%20Mesh%20Component%20Object%20Reference) (Animation :type Anim%20Sequence%20Base%20Object%20Reference) (TotalDuration :type Float%20%28single-precision%29) (EventReference :type Anim%20Notify%20Event%20Reference%20Structure%20%28by%20ref%29))
  (return false))

(fn ReceivedNotifyTick
  (params (MeshComp :type Skeletal%20Mesh%20Component%20Object%20Reference) (Animation :type Anim%20Sequence%20Base%20Object%20Reference) (FrameDeltaTime :type Float%20%28single-precision%29) (EventReference :type Anim%20Notify%20Event%20Reference%20Structure%20%28by%20ref%29))
  (bind _returnvalue (Transformation|GetSocketLocation MeshComp "hand_rSocket"))
  (bind (_outactors _returnvalue_2) (Collision|SphereOverlapActors MeshComp _returnvalue 1e+02 (Utilities|Array|MakeArray "ObjectTypeQuery3") "/Game/FPS_AnimBP_v2/Blueprints/BP_FPS_Character.BP_FPS_Character_C"))
  (if _returnvalue_2
    (for _array_element _outactors
      (bind _asbp_fps_character (Utilities|Casting|CastToBP_FPS_Character _array_element))
      (Character|LaunchCharacter _asbp_fps_character (Math|Vector|MakeVector (.X (Math|Vector|BreakVector (Math|Vector|ClampVectorSize (- (Transformation|GetActorLocation _array_element) _returnvalue) 1e+03 1e+03))) (.Y (Math|Vector|BreakVector (Math|Vector|ClampVectorSize (- (Transformation|GetActorLocation _array_element) _returnvalue) 1e+03 1e+03))) 2e+02) true false)
      (Game|Damage|ApplyDamage 0 1.0 0 0 "/Game/Blueprints/Damage/Damage_Giant/DBP_Hit.DBP_Hit_C")
      (return false))))

(fn ReceivedNotifyEnd
  (params (MeshComp :type Skeletal%20Mesh%20Component%20Object%20Reference) (Animation :type Anim%20Sequence%20Base%20Object%20Reference) (EventReference :type Anim%20Notify%20Event%20Reference%20Structure%20%28by%20ref%29))
  (return false))

(fn GetNotifyName
  (return "DoubleMediumAttack_2"))