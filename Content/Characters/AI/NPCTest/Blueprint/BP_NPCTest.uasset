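; BP_NPCTest is a test AI NPC character that reacts to damage and performs a melee attack.
; When damaged, it clears the investigating flag in its Blackboard and sets TargetLocation to the player's current location, whoever caused the damage.
; MeleeAttack plays a montage whose notify triggers a short sphere trace forward from the right-hand socket on the Camera channel, applying damage to the hit actor.
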(event EventBeginPlay)

(event EventMeleeAttack
  (bind _mesh (Variables|Character|GetMesh))
  (bind _returnvalue (Transformation|GetSocketLocation _mesh "hand_rSocket"))
  (Animation|Montage|PlayMontage (Variables|Character|GetMesh) "/Game/Characters/Mannequins/Animations/Manny/MM_MeleeAttack_Montage.MM_MeleeAttack_Montage"
    (:OnNotifyBegin
      (bind _outhit (Collision|SphereTraceByChannel _returnvalue (+ _returnvalue (* (Math|Vector|GetForwardVector (Transformation|GetActorRotation)) 5e+01)) 4e+01 "TraceTypeQuery2" false 0 "ForOneFrame"))
      (Game|Damage|ApplyDamage (.hitactor _outhit) 1.0 0 self))))

(event Game|Damage|EventAnyDamage
  (params (Damage :type Float%20%28single-precision%29) (DamageType :type Damage%20Type%20Object%20Reference) (InstigatedBy :type Controller%20Object%20Reference) (DamageCauser :type Actor%20Object%20Reference))
  (bind _returnvalue (Pawn|GetController))
  (bind _returnvalue_2 (AI|GetBlackboard _returnvalue))
  (AI|Components|Blackboard|SetValueasBool _returnvalue_2 (Utilities|Name|MakeLiteralName "bIsInvastigating") false)
  (AI|Components|Blackboard|SetValueasVector _returnvalue_2 (Utilities|Name|MakeLiteralName "TargetLocation") (Transformation|GetActorLocation (Game|GetPlayerCharacter 0))))

(fn ConstructionScript)