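; AI controller for the test NPC that runs BT_NPCTest and supplies its patrol and player-awareness blackboard data.
; On begin play it starts the tree, then seeds looping and wait time from the pawn's PatrolPath, plus an initial direction.
; AI perception updates set bAwarePlayer from whether the first-person character is successfully sensed; the branch after that is empty.
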(event OnTargetPerceptionUpdated(AIPerception)
  (params (Actor :type Actor%20Object%20Reference) (Stimulus :type AI%20Stimulus%20Structure))
  (bind _bsuccessfullysensed (Utilities|Struct|BreakAIStimulus Stimulus))
  (Utilities|Casting|CastToBP_FirstPersonCharacter Actor)
  (AI|Components|Blackboard|SetValueasBool (AI|GetBlackboard 0) (Utilities|Name|MakeLiteralName "bAwarePlayer") _bsuccessfullysensed)
  (if _bsuccessfullysensed
    _))

(event EventBeginPlay
  (bind _returnvalue (AI|GetBlackboard 0))
  (AI|RunBehaviorTree "/Game/Characters/AI/NPCTest/BT_NPCTest.BT_NPCTest")
  (bind _asbp_npctest (Utilities|Casting|CastToBP_NPCTest (Pawn|GetControlledPawn)))
  (bind _output_get (Variables|Default|SetMyPawn _asbp_npctest))
  (AI|Components|Blackboard|SetValueasBool _returnvalue (Utilities|Name|MakeLiteralName "bPathLooping") (Variables|/Game/Characters/AI/NPCTest/Blueprint/PatrolPath.PatrolPath_C|GetbIsLooping (Variables|/Game/Characters/AI/NPCTest/Blueprint/BP_NPCTest.BP_NPCTest_C|GetPatrolPath _output_get)))
  (Class|BlackboardComponent|SetValueasInt _returnvalue (Utilities|Name|MakeLiteralName "Direction") 1)
  (AI|Components|Blackboard|SetValueasFloat _returnvalue (Utilities|Name|MakeLiteralName "WaitTime") (Variables|/Game/Characters/AI/NPCTest/Blueprint/PatrolPath.PatrolPath_C|GetWatiTime (Variables|/Game/Characters/AI/NPCTest/Blueprint/BP_NPCTest.BP_NPCTest_C|GetPatrolPath _output_get))))

(fn ConstructionScript)