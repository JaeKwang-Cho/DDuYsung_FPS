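; Interactable prop that spawns batches of BP_PickupAmmo bricks of randomly rolled ammo categories around its spawn point.
; Interact clears any pending timer and calls SpawnAmmo, which chains randomly offset drops on a short timer until the batch count or live-pickup cap is reached.
; Each pickup's OnPickup event is bound on spawn to track the live count.
; The construction script clamps batch size and toggles the platform and light.
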(event EventOnAmmoPickedUp
  (Variables|Default|SetTotalCurrentAmmoPickups (Math|Integer|Clamp(Integer) (- (Variables|Default|GetTotalCurrentAmmoPickups) 1) 0 (Variables|Default|GetMaxLiveAmmoPickups))))

(event EventBeginPlay)

(event EventInteract
  (params (InteractingActor :type Actor%20Object%20Reference))
  (if (Utilities|Time|IsValidTimerHandle (Variables|Default|GetSpawnTimer))
    (Utilities|Time|ClearandInvalidateTimerbyHandle (Variables|Default|GetSpawnTimer)))
  (CallFunction|SpawnAmmo))

(fn ConstructionScript
  (bind _sm_base2 (Variables|Default|GetSM_Base2))
  (bind _pointlight (Variables|Default|GetPointLight))
  (|CallParentFunction)
  (Variables|Default|SetAmmoDropsToSpawn (Math|Integer|Clamp(Integer) (Variables|Default|GetAmmoDropsToSpawn) 1 10))
  (Development|SetHiddeninGame _sm_base2 (not (Variables|Default|GetShowPlatform)) false)
  (Rendering|SetVisibility _sm_base2 (Variables|Default|GetShowPlatform) false)
  (Development|SetHiddeninGame _pointlight (not (Variables|Default|GetShowSpotlight)) false)
  (Rendering|SetVisibility _pointlight (Variables|Default|GetShowSpotlight) false))

(fn SpawnAmmo
  (bind _ammo_data_asset (CallFunction|RollforAmmoCategory))
  (bind _spawnlocation (Variables|Default|GetSpawnLocation))
  (bind _returnvalue (Transformation|GetWorldTransform _spawnlocation))
  ;[0 0 0] Attempt to spawn a specified amount of ammo bricks of a random ammo category, each with a slight location offset
  (if (< (Variables|Default|GetTotalCurrentAmmoPickups) (Variables|Default|GetMaxLiveAmmoPickups))
    (Utilities|IsValid _ammo_data_asset
      (:Is%20Valid
        (bind _returnvalue_2 (Game|SpawnActorfromClass "/Game/FPS_AnimBP_v2/Blueprints/Pickups/BP_PickupAmmo.BP_PickupAmmo_C" (Math|Transform|MakeTransform (+ (Math|Vector|MakeVector (Math|Random|RandomFloatinRange -5e+01 5e+01) (Math|Random|RandomFloatinRange -5e+01 5e+01) 0.0) (.location _returnvalue)) (.rotation _returnvalue) "1.000000,1.000000,1.000000") "AdjustIfPossibleButAlwaysSpawn" 0 _ammo_data_asset 0 true false 0.0 "(R=1.000000,G=1.000000,B=1.000000,A=1.000000)" 0))
        (EventDispatchers|BindEventtoOnPickup _returnvalue_2 (EventDispatchers|CreateEvent :!event OnAmmoPickedUp))
        (Math|Integer|IncrementInt (Variables|Default|GetTotalCurrentAmmoPickups)
          (:%20%20
            (bind _result (Math|Integer|IncrementInt (Variables|Default|GetAmmoDropsSpawned))
              (:%20%20
                (if (< _result (Variables|Default|GetAmmoDropsToSpawn))
                  (bind _returnvalue_3 (Utilities|Time|SetTimerbyEvent (EventDispatchers|CreateEvent :!event SpawnAmmo) 0.25))
                  (Variables|Default|SetSpawnTimer _returnvalue_3)
                  (else
                    (Variables|Default|SetAmmoDropsSpawned 0))))))))
      (:Is%20Not%20Valid
        (|PrintErrorInvalidAmmoCategory)))))