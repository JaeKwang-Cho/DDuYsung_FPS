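; Grenade projectile child Blueprint that runs a fuse timer from BeginPlay and ignores bounce and stop events, suggesting timed detonation.
; Detonate plays explosion sound, camera shake and particles, calls ApplyDamageAndImpulse, spawns shrapnel, then destroys the actor.
; ApplyDamageAndImpulse pushes physics-simulating sphere-trace hits with distance-scaled impulses, then applies radial damage.
; The CalculateShrapnelTransform override randomizes shrapnel position and direction around the grenade in all directions.
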(event OnProjectileStop(Projectile)
  (params (ImpactResult :type Hit%20Result%20Structure%20%28by%20ref%29))
  ;[0 0 0] Override these to do nothing
)

(event OnProjectileBounce(Projectile)
  (params (ImpactResult :type Hit%20Result%20Structure%20%28by%20ref%29) (ImpactVelocity :type Vector%20%28by%20ref%29 :default "0, 0, 0"))
  ;[0 0 0] Override these to do nothing
)

(event EventBeginPlay
  ;[0 0 0] Count down the fuse timer until detonation
  (|CallParentFunction)
  (Utilities|Time|SetTimerbyEvent (EventDispatchers|CreateEvent :!event Detonate) (Variables|Default|GetFuseTimer)))

(event EventTick
  (params (DeltaSeconds :type Float%20%28single-precision%29))
  ;[0 0 0] Override these to do nothing
)

(fn ConstructionScript
  (|CallParentFunction))

(fn Detonate
  (bind _damageradius (Variables|Default|GetDamageRadius))
  (bind _projectilecollision (Variables|Default|GetProjectileCollision))
  (bind _returnvalue (Transformation|GetWorldLocation _projectilecollision))
  ;[0 0 0] Call an override of Apply Damage and Impulse
  (Audio|PlaySoundatLocation (Variables|Default|GetExplosionSound) _returnvalue "0, 0, 0" 1.0 1.0 0.0 0 0 0 0)
  (Camera|PlayWorldCameraShake "/Game/FPS_AnimBP_v2/Blueprints/Camera/CameraShakes/BP_ShakeExplosion.BP_ShakeExplosion_C" _returnvalue _damageradius (* _damageradius 2.0))
  (Effects|SpawnEmitteratLocation "/Game/FPS_AnimBP_v2/Demo/UE5/ExampleContent/Effects/P_Explosion_Bomb.P_Explosion_Bomb" _returnvalue "0, 0, 0" "1.000000,1.000000,1.000000" true "AutoRelease")
  (CallFunction|ApplyDamageandImpulse)
  (CallFunction|SpawnShrapnel)
  (Actor|DestroyActor))

(fn ApplyDamageandImpulse
  (LocalVariables|Setlocal_Origin (Transformation|GetWorldLocation (Variables|Default|GetProjectileCollision)))
  (Utilities|FlowControl|Sequence
    (:then_0
      ;[0 0 0] Apply a radial impulse to any targets caught in the explosion based on their direction and distance from the center
      (bind _outhits (Collision|MultiSphereTraceByChannel (LocalVariables|Getlocal_Origin) (LocalVariables|Getlocal_Origin) (Variables|Default|GetDamageRadius) "TraceTypeQuery1" false 0 "None"))
      (for _array_element _outhits
        (if (Physics|IsSimulatingPhysics (.HitComponent (Collision|BreakHitResult _array_element)) "None")
          (bind _output_get (LocalVariables|Setlocal_Distance (- (.ImpactPoint (Collision|BreakHitResult _array_element)) (LocalVariables|Getlocal_Origin))))
          (Physics|AddImpulseatLocation (.HitComponent (Collision|BreakHitResult _array_element)) (* (Math|Vector|Normalize _output_get) (* (Math|Float|Power (/ (Variables|Default|GetDamageRadius) (Math|Vector|VectorLength (LocalVariables|Getlocal_Distance))) 0.4) 3e+05)) (.Location (Collision|BreakHitResult _array_element)) "None"))))
    (:then_1
      ;[0 0 0] Apply Radial damage
      (Game|Damage|ApplyRadialDamage (Variables|Default|GetBaseDamage) (LocalVariables|Getlocal_Origin) (Variables|Default|GetDamageRadius) (Variables|Default|GetDamageType) 0 self (Variables|Default|GetOwningController) false "ECC_Visibility"))))

(fn CalculateShrapnelTransform
  (bind _projectilecollision (Variables|Default|GetProjectileCollision))
  (bind _returnvalue (Transformation|GetWorldLocation _projectilecollision))
  (bind _returnvalue_2 (Math|Random|RandomUnitVectorinConeinDegrees _returnvalue 1.8e+02))
  ;[0 0 0] Override the shrapnel direction calculation for the explosion
  (return (Math|Transform|MakeTransform (+ _returnvalue (* _returnvalue_2 5.0)) (Math|Rotator|MakeRotfromX _returnvalue_2) "1.000000,1.000000,1.000000")))