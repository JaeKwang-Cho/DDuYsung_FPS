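; Base projectile actor for FPS weapons, configured from a ProjectileDataAsset during construction.
; On bounce it plays impact sound and decal, applies damage and impulse, rolls for shrapnel child projectiles, then ricochets or stops and is destroyed.
; Tick aligns and scales the tracer by velocity and plays a fly-by sound for the Instigator; fly-by overlaps also report AI noise.
; Homing and penetration settings load but are marked unimplemented.
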(event OnComponentEndOverlap(FlyByDetection)
  (params (OverlappedComponent :type Primitive%20Component%20Object%20Reference) (OtherActor :type Actor%20Object%20Reference) (OtherComp :type Primitive%20Component%20Object%20Reference) (OtherBodyIndex :type Integer))
  ;[0 0 0] Player is no longer in range
  (Utilities|IsValid OtherActor
    (:Is%20Valid
      (if (== OtherActor (Variables|Actor|GetInstigator))
        (Variables|LiveData|SetCharacterIsInFlyByRange false)))))

(event OnComponentBeginOverlap(FlyByDetection)
  (params (OverlappedComponent :type Primitive%20Component%20Object%20Reference) (OtherActor :type Actor%20Object%20Reference) (OtherComp :type Primitive%20Component%20Object%20Reference) (OtherBodyIndex :type Integer) (bFromSweep :type Boolean) (SweepResult :type Hit%20Result%20Structure%20%28by%20ref%29))
  ;[0 0 0] Players and Enemies can hear bullets that pass close by them
  (Utilities|IsValid OtherActor
    (:Is%20Valid
      (Utilities|FlowControl|Sequence
        (:then_0
          (if (== (Variables|Actor|GetInstigator) OtherActor)
            (Variables|LiveData|SetCharacterIsInFlyByRange true)))
        (:then_1
          (if (Variables|/Script/Engine.Actor|GetbCanBeDamaged OtherActor)
            (Class|AISenseHearing|ReportNoiseEvent (Transformation|GetActorLocation) (Variables|FlyBy|GetFlyByLoudness) (Variables|Actor|GetInstigator) (Variables|FlyBy|GetFlyByDetectionRadius) "None")))))))

(event OnProjectileBounce(Projectile)
  (params (ImpactResult :type Hit%20Result%20Structure%20%28by%20ref%29) (ImpactVelocity :type Vector%20%28by%20ref%29 :default "0, 0, 0"))
  ;[0 0 0] Save the impact values, play the impact sound, damage the hit target
  (Impact|SetImpactValues ImpactResult ImpactVelocity)
  (Impact|ImpactFX)
  (Impact|ApplyDamageandImpulse)
  (Shrapnel|SpawnShrapnel)
  (Ricochet|HandleRicochet))

(event OnProjectileStop(Projectile)
  (params (ImpactResult :type Hit%20Result%20Structure%20%28by%20ref%29))
  ;[0 0 0] Destroy this projectile when it is stopped
  (Actor|DestroyActor))

(event EventBeginPlay
  ;[0 0 0] Begin Play - Determine if the player is in front of or behind the projectile
  (Variables|LiveData|SetSpawnLocation (Transformation|GetActorLocation))
  (if (>= (FlyBy|GetAngletoPlayer) 9e+01)
    (Variables|LiveData|SetCharacterIsInFront false)
    (else
      (Variables|LiveData|SetCharacterIsInFront true))))

(event EventTick
  (params (DeltaSeconds :type Float%20%28single-precision%29))
  ;[0 0 0] Event Tick - Fly By Effects
  (Projectile|UpdateBulletRotationandScale)
  (FlyBy|Flyby))

(fn ConstructionScript
  (Initialisation|InitialiseProjectile))

(fn GetAngletoPlayer
  ;[0 0 0] 0 = In Front
  ; 90 = Next to
  ; 180 = Behind
  (return (Class|KismetMathLibrary|DegAcos (Class|Actor|GetDotProductto (Variables|Actor|GetInstigator)))))

(fn Flyby
  ;[0 0 0] Play the Fly By sound effect if the projectile is moving towards the player as it passes
  (if (Math|Boolean|ANDBoolean (Variables|LiveData|GetCharacterIsInFlyByRange) (Variables|LiveData|GetCharacterIsInFront) (Variables|FlyBy|GetPlayFlyBySound))
    (if (>= (FlyBy|GetAngletoPlayer) 9e+01)
      (Utilities|FlowControl|DoOnce false
        (:Completed
          (Audio|PlaySoundatLocation (Variables|FlyBy|GetFlyBySound) (Transformation|GetWorldLocation (Variables|Default|GetFlyByDetection)) "0, 0, 0" 1.0 1.0 0.0 0 0 0 0))))))

(fn ScaleBulletTracer
  ;[0 0 0] Scale the bullet tracer mesh based on velocity
  (Transformation|SetWorldScale3D (Variables|Components|GetBulletTracer) (Math|Vector|Lerp(Vector) "0.025000,0.010000,0.010000" "0.300000,0.010000,0.010000" (Math|Float|MapRangeClamped (Math|Vector|VectorLength (Transformation|GetVelocity)) 0.0 1e+04 0.0 1.0))))

(fn UpdateBulletRotationandScale
  (bind _returnvalue (Transformation|GetActorLocation))
  ;[0 0 0] Update the projectile's rotation based on direction
  (Transformation|SetWorldRotation (Variables|Default|GetProjectileCollision) (Math|Rotator|FindLookatRotation _returnvalue (+ _returnvalue (Transformation|GetVelocity))) false false)
  (Projectile|ScaleBulletTracer))

(fn HandleRicochet
  ;[0 0 0] Handle whether this shot can ricochet based on permission, chance, number of bounces and impact angle
  (if (Ricochet|CalculateRichocetOddsandAngle)
    (if (< (Variables|LiveData|GetCurrentNumberOfBounces) (Variables|Projectile|GetMaxBounces))
      (Math|Integer|IncrementInt (Variables|LiveData|GetCurrentNumberOfBounces)
        (:%20%20
          (Ricochet|Ricochet)))
      (else
        (Components|Movement|StopMovementImmediately (Variables|Components|GetProjectile) :!label _label)))
    (else
      (goto _label))))

(fn CalculateRichocetOddsandAngle
  (return (Default|CalculateRicochetOddsandAngle (Variables|Initialisation|GetProjectileDataAsset) (Variables|LiveData|GetImpactResult) (Variables|LiveData|GetImpactVector))))

(fn SetImpactValues
  (params (ImpactResult :type Hit%20Result%20Structure) (InputPin :type Vector%20%28by%20ref%29))
  ;[0 0 0] Set the live impact values when the projectile impacts something
  (Variables|LiveData|SetImpactResult ImpactResult)
  (Variables|LiveData|SetImpactVelocity InputPin)
  (Variables|LiveData|SetImpactVector (Transformation|GetVelocity))
  (Variables|LiveData|SetImpactTransform (Transformation|GetWorldTransform (Variables|Default|GetProjectileCollision)))
  (Variables|LiveData|SetImpactSurfaceType (Variables|/Script/PhysicsCore.PhysicalMaterial|GetSurfaceType (.PhysMat (Collision|BreakHitResult (Variables|LiveData|GetImpactResult))))))

(fn ApplyDamageandImpulse
  (LocalVariables|Setlocal_ImpactPoint (.ImpactPoint (Collision|BreakHitResult (Variables|LiveData|GetImpactResult))))
  ;[0 0 0] Apply a physics impulse on hit if the hit component is simulating physics and apply damage if the hit object can take damage
  (Default|ApplyImpactImpulse (Variables|Initialisation|GetProjectileDataAsset) (Variables|LiveData|GetImpactVelocity) (Variables|LiveData|GetImpactResult))
  (Default|ApplyPointDamage (Variables|Initialisation|GetProjectileDataAsset) (Variables|LiveData|GetImpactResult) (Variables|LiveData|GetSpawnLocation) (LocalVariables|Getlocal_ImpactPoint) (Variables|Initialisation|GetOwningController) (Variables|Actor|GetInstigator) (Variables|Damage|GetDamageType) (Variables|Damage|GetBaseDamage) (Variables|Damage|GetMaxEffectiveRange) (Variables|Damage|GetDropOffCurve)))

(fn CalculateDamageDropOff
  ;[0 0 0] Calculate the damage on hit
  (return (Default|CalculateDamage (Variables|Initialisation|GetProjectileDataAsset) (Variables|LiveData|GetImpactResult) (Variables|LiveData|GetSpawnLocation) (Variables|Damage|GetBaseDamage) (Variables|Damage|GetMaxEffectiveRange) (Variables|Damage|GetDropOffCurve))))

(fn ImpactFX
  (bind _impactresult (Variables|LiveData|GetImpactResult))
  (bind (_bblockinghit _binitialoverlap _time _distance _location _impactpoint _normal _impactnormal _physmat _hitactor _hitcomponent) (Collision|BreakHitResult _impactresult))
  ;[0 0 0] Apply the impact effects such as sounds and decals on impact
  (Audio|PlaySoundatLocation (Variables|Impact|GetImpactSound) _location "0, 0, 0" 1.0 1.0 0.0 0 0 0 0)
  (Class|GameplayStatics|SpawnDecalAttached "/Game/FPS_AnimBP_v2/Materials/M_Decal.M_Decal" "0.100000,10.000000,10.000000" _hitcomponent "None" _impactpoint (Math|Rotator|MakeRotfromX _impactnormal) "KeepWorldPosition" 1e+01))

(fn InitialiseProjectile
  ;[0 0 0] Initialise all the projectile settings
  (Initialisation|SetInitialisationSettings)
  (Initialisation|SetProjectileSettings)
  (Initialisation|SetFlybySettings)
  (Initialisation|SetHomingSettings)
  (Initialisation|SetImpactSettings)
  (Initialisation|SetRicochetSettings)
  (Initialisation|SetPenetrationSettings)
  (Initialisation|SetShrapnelSettings))

(fn SetInitialisationSettings
  (bind _particlesystem (Variables|Default|GetParticleSystem))
  ;[0 0 0] Get the Initialisation Data from the data asset and set those settings
  (bind (_staticmesh _particlesystem_2 _projectiletype) (Default|GetInitialisationData (Variables|Initialisation|GetProjectileDataAsset)))
  (Components|StaticMesh|SetStaticMesh (Variables|Components|GetBulletTracer) _staticmesh)
  (Effects|Components|ParticleSystem|SetTemplate (Variables|Default|GetParticleSystem) _particlesystem_2)
  (Variables|Initialisation|SetProjectileType _projectiletype)
  (Utilities|IsValid (Variables|/Script/Engine.ParticleSystemComponent|GetTemplate _particlesystem)
    (:Is%20Valid
      (Components|Activation|Activate _particlesystem true))))

(fn SetProjectileSettings
  (bind _projectile (Variables|Components|GetProjectile))
  (bind _projectile_2 (Variables|Components|GetProjectile))
  ;[0 0 0] Get the Projectile data from the data asset and set those settings
  (bind (_lifespan _projectileradius _initialprojectilespeed _maxprojectilespeed _gravityenabled _gravityscale _shouldbounce _maxbounces) (Default|GetProjectileSettings (Variables|Initialisation|GetProjectileDataAsset)))
  (Actor|SetLifeSpan _lifespan)
  (Components|Sphere|SetSphereRadius (Variables|Default|GetProjectileCollision) _projectileradius true)
  (Variables|/Script/Engine.ProjectileMovementComponent|SetInitialSpeed _projectile _initialprojectilespeed)
  (Variables|/Script/Engine.ProjectileMovementComponent|SetMaxSpeed _projectile _maxprojectilespeed)
  (Physics|SetEnableGravity (Variables|Default|GetProjectileCollision) _gravityenabled)
  (Variables|/Script/Engine.ProjectileMovementComponent|SetProjectileGravityScale _projectile_2 _gravityscale)
  (Variables|/Script/Engine.ProjectileMovementComponent|SetbShouldBounce _projectile_2 _shouldbounce)
  (Variables|Projectile|SetMaxBounces _maxbounces))

(fn SetFlybySettings
  ;[0 0 0] Get the Fly By data from the data asset and set those settings
  (bind (_enableflybydetection _playflybysound _flybysound _flybydetectionradius _flybyloudness) (Default|GetFlybySettings (Variables|Initialisation|GetProjectileDataAsset)))
  (Variables|FlyBy|SetEnableFlyByDetection _enableflybydetection)
  (Variables|FlyBy|SetPlayFlyBySound _playflybysound)
  (Variables|FlyBy|SetFlyBySound _flybysound)
  (Components|Sphere|SetSphereRadius (Variables|Default|GetFlyByDetection) _flybydetectionradius true)
  (Variables|FlyBy|SetFlyByLoudness _flybyloudness))

(fn SetHomingSettings
  (bind _projectile (Variables|Components|GetProjectile))
  ;[0 0 0] Get the Homing data from the data asset and set those settings. Homing is not currently implemented
  (bind (_enablehomingprojectile _homingacceleration _homingstartdelay) (Default|GetHomingSettings (Variables|Initialisation|GetProjectileDataAsset)))
  (Variables|/Script/Engine.ProjectileMovementComponent|SetbIsHomingProjectile _projectile _enablehomingprojectile)
  (Variables|/Script/Engine.ProjectileMovementComponent|SetHomingAccelerationMagnitude _projectile _homingacceleration)
  (Variables|Homing|SetHomingStartDelay _homingstartdelay))

(fn SetImpactSettings
  ;[0 0 0] Get the Impact data from the data asset and set those settings
  (bind (_impactdecal _impactsound _applyimpulseonhit _impactforcestrength _impactalertrange _impactloudness) (Default|GetImpactSettings (Variables|Initialisation|GetProjectileDataAsset)))
  (Variables|Impact|SetImpactDecal _impactdecal)
  (Variables|Impact|SetImpactSound _impactsound)
  (Variables|Impact|SetApplyImpulseOnHit _applyimpulseonhit)
  (Variables|Impact|SetImpactForceStrength _impactforcestrength)
  (Variables|Impact|SetImpactAlertRange _impactalertrange)
  (Variables|Impact|SetImpactLoudness _impactloudness))

(fn SetRicochetSettings
  ;[0 0 0] Get the Ricochet data from the data asset and set those settings
  (bind (_enablericochet _ricochetsound _maxricochetchance) (Default|GetRicochetSettings (Variables|Initialisation|GetProjectileDataAsset)))
  (Variables|Ricochet|SetEnableRicochet _enablericochet)
  (Variables|Ricochet|SetRicochetSound _ricochetsound)
  (Variables|Ricochet|SetMaxRicochetChance _maxricochetchance))

(fn SetPenetrationSettings
  ;[0 0 0] Get the Penetration data from the data asset and set those settings. Penetration is not currently implemented
  (bind (_enablepenetration _maxpenetratedobjects _penetrationstrength) (Default|GetPenetrationSettings (Variables|Initialisation|GetProjectileDataAsset)))
  (Variables|Penetration|SetEnablePenetration _enablepenetration)
  (Variables|Penetration|SetMaxPenetratedObjects _maxpenetratedobjects)
  (Variables|Penetration|SetPenetrationSrength _penetrationstrength))

(fn SetShrapnelSettings
  ;[0 0 0] Get the Shrapnel data from the data asset and set those settings
  (bind (_enableshrapnel _shrapnelclass _shrapnelchance _shrapnelchanceaffectedbyimpactangle _numberofshrapnelmax) (Default|GetShrapnelSettings (Variables|Initialisation|GetProjectileDataAsset)))
  (Variables|Shrapnel|SetEnableShrapnel _enableshrapnel)
  (Variables|Shrapnel|SetShrapnelDataAsset _shrapnelclass)
  (Variables|Shrapnel|SetShrapnelChance _shrapnelchance)
  (Variables|Shrapnel|SetShrapnelChanceAffectedByImpactAngle _shrapnelchanceaffectedbyimpactangle)
  (Variables|Shrapnel|SetNumberOfShrapnelMax _numberofshrapnelmax))

(fn SpawnShrapnel
  ;[0 0 0] Handle spawning the shrapnel based on chance
  (if (Variables|Shrapnel|GetEnableShrapnel)
    (for _index (range 0 (Variables|Shrapnel|GetNumberOfShrapnelMax))
      (if (< (Math|Random|RandomFloat) (Variables|Shrapnel|GetShrapnelChance))
        (Game|SpawnActorfromClass (Default|GetProjectileClass (Variables|Shrapnel|GetShrapnelDataAsset)) (Default|CalculateShrapnelTransform (Variables|Initialisation|GetProjectileDataAsset) (Variables|LiveData|GetImpactResult) (Variables|LiveData|GetImpactVector)) "AdjustIfPossibleButAlwaysSpawn" 0 (Variables|Shrapnel|GetShrapnelDataAsset) (Variables|Initialisation|GetOwningWeapon) (Variables|Initialisation|GetOwningController) (Variables|Damage|GetDamageType) 1e+01 5e+02 "/Game/FPS_AnimBP_v2/Data/Curves/CURVE_BulletDropOff.CURVE_BulletDropOff" (Variables|Actor|GetInstigator))))))

(fn CalculateShrapnelTransform
  (bind _impactresult (Variables|LiveData|GetImpactResult))
  (bind _impactvector (Variables|LiveData|GetImpactVector))
  (bind _projectile (Variables|Components|GetProjectile))
  (bind _impactvector_2 (Variables|LiveData|GetImpactVector))
  (bind _impactresult_2 (Variables|LiveData|GetImpactResult))
  (bind _impactnormal (Collision|BreakHitResult _impactresult))
  (bind _returnvalue (Math|Vector|Normalize _impactvector_2))
  (bind _impactnormal_2 (Collision|BreakHitResult _impactresult_2))
  (bind _initialspeed (Variables|/Script/Engine.ProjectileMovementComponent|GetInitialSpeed _projectile))
  (bind _returnvalue_2 (Math|Vector|MirrorVectorbyNormal _returnvalue _impactnormal_2))
  (bind _returnvalue_3 (* _impactnormal -1))
  (bind _returnvalue_4 (Math|Vector|DotProduct _impactvector _returnvalue_3))
  (bind _returnvalue_5 (/ _returnvalue_4 _initialspeed))
  (bind _returnvalue_6 (Math|Float|MapRangeClamped _returnvalue_5 0.0 1.0 5.0 6e+01))
  (bind _returnvalue_7 (Math|Random|RandomUnitVectorinConeinDegrees _returnvalue_2 _returnvalue_6))
  ;[0 0 0] Calculate the chance of shrapnel spwaning based on the impact vector
  (return (Math|Transform|MakeTransform (+ (.location (Variables|LiveData|GetImpactTransform)) (* _returnvalue_7 5.0)) (Math|Rotator|MakeRotfromX _returnvalue_7) "1.000000,1.000000,1.000000")))

(fn Ricochet
  ;[0 0 0] Play the ricochet sound
  (Audio|PlaySoundatLocation (Variables|Ricochet|GetRicochetSound) (.location (Variables|LiveData|GetImpactTransform)) "0, 0, 0" 1.0 1.0 0.0 0 0 0 0))