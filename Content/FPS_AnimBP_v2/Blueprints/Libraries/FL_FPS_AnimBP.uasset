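; Blueprint function library of shared helpers for an FPS project, covering error printing, input device tracking, HUD access and weapon attachment checks.
; Input device and HUD helpers send messages to player controller 0, while a separate helper classifies keys as keyboard/mouse or gamepad.
; Error messages are colored by urgency.
; Attachment checks honor allowed-gun lists (empty allows all) and block by exclusion only when both slot and specific attachment are disallowed.
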(fn PrintErrorMessage
  (params (Message :type String) (Self%20Object :type Object%20Object%20Reference) (Function%20Name :type String) (Urgency :type E_ErrorMessageUrgency%20Enum :default "NewEnumerator0") (bPrintToScreen :type Boolean) (bPrintToLog :type Boolean) (Duration :type Float%20%28double-precision%29))
  ;[0 0 0] Prints a unified error message with the class and function named specified if desired
  (LocalVariables|Setlocal_String (Utilities|String|Append Message " 
" (Utilities|GetClassDisplayName (Utilities|GetClass Self%20Object)) " > " Function%20Name))
  (LocalVariables|Setlocal_TextColor (Utilities|Select :Index Urgency :NewEnumerator0 "(R=0.636880,G=1.000000,B=0.000000,A=1.000000)" :NewEnumerator1 "(R=1.000000,G=0.442751,B=0.000000,A=1.000000)" :NewEnumerator2 "(R=1.000000,G=0.000000,B=0.000000,A=1.000000)"))
  (Development|PrintString 0 (LocalVariables|Getlocal_String) bPrintToScreen bPrintToLog (LocalVariables|Getlocal_TextColor) Duration))

(fn GetCurrentInputDevice
  (bind _inputdevice (Class|BPControllerInterface|GetInputDevice(Message) (Game|GetPlayerController 0)))
  (return _inputdevice))

(fn UpdateInputDevice
  (params (Key :type Key%20Structure :default "None"))
  (Class|BPControllerInterface|OnAnyKeyPress(Message) (Game|GetPlayerController 0) Key))

(fn GetPlayerHUD
  (bind _gameplayhud (Class|BPControllerInterface|GetGameplayHUD(Message) (Game|GetPlayerController 0)))
  (return _gameplayhud))

(fn GetInputDevicebyKey
  (params (Key :type Key%20Structure%20%28by%20ref%29))
  ;[0 0 0] Get the current input device based on the last input recieved
  (if (or (Class|KismetInputLibrary|KeyIsKeyboardKey Key) (Class|KismetInputLibrary|KeyIsMouseButton Key))
    (return "NewEnumerator0")
    (elif (Class|KismetInputLibrary|KeyIsGamepadKey Key)
      (return "NewEnumerator1"))))

(fn IsWeaponAttachmentAllowed
  (params (AttachmentDataAsset :type FPS%20PDA%20Attachment%20Data%20Base%20Object%20Reference) (WeaponAttachments :type ST%20Weapon%20Attachments%20Structure%20%28by%20ref%29) (Gun%20Data%20Asset :type FPS%20PDA%20Gun%20Base%20Object%20Reference))
  (bind (_disallowedattachmentslots _disallowedspecificattachments) (Utilities|Struct|BreakST_WeaponAttachments WeaponAttachments))
  (bind _allowedguns (Variables|/Game/FPS_AnimBP_v2/Blueprints/DataAssets/Attachments/FPS_PDA_AttachmentDataBase.FPS_PDA_AttachmentDataBase_C|GetAllowedGuns AttachmentDataAsset))
  ;[0 0 0] Check to see if the attachment is allowed to be equipped on this weapon
  (Utilities|IsValid AttachmentDataAsset
    (:Is%20Valid
      (return (and (or (not (Utilities|Set|Contains _disallowedattachmentslots (.AttachmentSlot (Default|GetAttachmentBaseData AttachmentDataAsset)))) (not (Utilities|Set|Contains _disallowedspecificattachments AttachmentDataAsset))) (or (== (Utilities|Array|Length _allowedguns) 0) (Utilities|Array|ContainsItem _allowedguns Gun%20Data%20Asset)))))
    (:Is%20Not%20Valid
      (return false))))